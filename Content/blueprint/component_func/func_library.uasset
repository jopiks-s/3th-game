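; Blueprint function library with a look-at rotation helper and small array checks for membership and non-emptiness.
; Rotate steps an actor root or component, optionally measured from a socket, at constant speed toward a position, or a target actor when that is zero.
; RotateType picks which axes are applied; Anim mode applies none.
; It returns the interpolated rotation and a done flag, and prints debug rotations on every call.
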(fn Rotate
  (params (actor%20rotate :type Actor%20Object%20Reference) (component%20rotate :type Skeletal%20Mesh%20Component%20Object%20Reference) (actor%20target :type Actor%20Object%20Reference) (position%20target%28priority%29 :type Vector) (socket%20name :type String) (rotate%20speed%20 :type Float%20%28single-precision%29) (what%20rotate :type what_rotate%20Enum :default "NewEnumerator0") (rotate%20type :type rotate_type%20Enum :default "NewEnumerator0"))
  (Utilities|FlowControl|Sequence
    (:then_0
      (switch Utilities|FlowControl|Switch|Switchonwhat_rotate what%20rotate
        (:NewEnumerator0
          (LocalVariables|Setrotate%20target (Variables|/Script/Engine.Actor|GetRootComponent actor%20rotate)))
        (:NewEnumerator1
          (LocalVariables|Setrotate%20target component%20rotate :!label _label))
        (:NewEnumerator2
          (goto _label))))
    (:then_1
      (LocalVariables|Getrotate%20target
        (:then
          (Utilities|FlowControl|Sequence
            (:then_0
              (if (Class|KismetMathLibrary|EqualExactlyVectorVector position%20target%28priority%29 "0, 0, 0")
                (LocalVariables|Setlook%20target (Transformation|GetActorLocation actor%20target))
                (else
                  (LocalVariables|Setlook%20target position%20target%28priority%29))))
            (:then_1
              (if (Utilities|Array|IsEmpty socket%20name)
                (LocalVariables|Setstart%20interp%20rotate (Transformation|GetWorldRotation (LocalVariables|Getrotate%20target)))
                (LocalVariables|Setstart%20position (Transformation|GetWorldLocation (LocalVariables|Getrotate%20target)))
                (else
                  (LocalVariables|SetSocketName (Utilities|String|StringToName socket%20name))
                  (LocalVariables|Setstart%20interp%20rotate (Transformation|GetSocketRotation (LocalVariables|Getrotate%20target) (LocalVariables|GetSocketName)))
                  (LocalVariables|Setstart%20position (Transformation|GetSocketLocation (LocalVariables|Getrotate%20target) (LocalVariables|GetSocketName))))))
            (:then_2
              (Development|PrintString 0 (Utilities|String|ToString(Rotator) (LocalVariables|Getstart%20interp%20rotate)) true true "(R=0.000000,G=0.660000,B=1.000000,A=1.000000)" 0.1)
              (Development|PrintString 0 (Utilities|String|ToString(Rotator) (Math|Rotator|FindLookatRotation (LocalVariables|Getstart%20position) (LocalVariables|Getlook%20target))) true true "(R=0.000000,G=1.000000,B=0.144610,A=1.000000)" 0.1)
              (bind _output_get (LocalVariables|SetInterp%20Output (Class|KismetMathLibrary|RInterptoConstant (LocalVariables|Getstart%20interp%20rotate) (Math|Rotator|FindLookatRotation (LocalVariables|Getstart%20position) (LocalVariables|Getlook%20target)) (Utilities|Time|GetWorldDeltaSeconds (LocalVariables|Get__WorldContext)) rotate%20speed%20)))
              (LocalVariables|Setz%20interp (.yaw _output_get))
              (LocalVariables|Setroll%20interp (.roll _output_get))
              (LocalVariables|Setpitch%20interp (.pitch _output_get))
              (if (Utilities|Enum|NotEqual(Enum) what%20rotate "NewEnumerator2")
                (switch Utilities|FlowControl|Switch|Switchonrotate_type rotate%20type
                  (:NewEnumerator0
                    (Transformation|SetWorldRotation (LocalVariables|Getrotate%20target) (Math|Rotator|MakeRotator (LocalVariables|Getroll%20interp) (LocalVariables|Getpitch%20interp) (LocalVariables|Getz%20interp)) false false))
                  (:NewEnumerator1
                    (Transformation|SetWorldRotation (LocalVariables|Getrotate%20target) (Math|Rotator|MakeRotator (LocalVariables|Getroll%20interp) 0.0 (LocalVariables|Getz%20interp)) false false)
                    (LocalVariables|Setdone%20rotate (Math|Vector|Equal(Vector) (Math|Vector2D|MakeVector2D (.pitch (LocalVariables|GetInterp%20Output)) (.yaw (LocalVariables|GetInterp%20Output))) (Math|Vector2D|MakeVector2D (.pitch (Math|Rotator|FindLookatRotation (LocalVariables|Getstart%20position) (LocalVariables|Getlook%20target))) (.yaw (Math|Rotator|FindLookatRotation (LocalVariables|Getstart%20position) (LocalVariables|Getlook%20target)))) 1.0)))
                  (:NewEnumerator3
                    (Transformation|SetWorldRotation (LocalVariables|Getrotate%20target) (Math|Rotator|MakeRotator 0.0 0.0 (LocalVariables|Getz%20interp)) false false)
                    (LocalVariables|Setdone%20rotate (== (LocalVariables|Getz%20interp) (.yaw (Math|Rotator|FindLookatRotation (LocalVariables|Getstart%20position) (LocalVariables|Getlook%20target))))))
                  (:NewEnumerator2
                    (Transformation|SetWorldRotation (LocalVariables|Getrotate%20target) (Math|Rotator|MakeRotator (LocalVariables|Getroll%20interp) 0.0 0.0) false false)
                    (LocalVariables|Setdone%20rotate (== (LocalVariables|Getroll%20interp) (.roll (Math|Rotator|FindLookatRotation (LocalVariables|Getstart%20position) (LocalVariables|Getlook%20target)))))))
                (else
                  (switch Utilities|FlowControl|Switch|Switchonrotate_type rotate%20type
                    (:NewEnumerator1
                      (LocalVariables|Setdone%20rotate (Math|Vector|Equal(Vector) (Math|Vector2D|MakeVector2D (.pitch (LocalVariables|GetInterp%20Output)) (.yaw (LocalVariables|GetInterp%20Output))) (Math|Vector2D|MakeVector2D (.pitch (Math|Rotator|FindLookatRotation (LocalVariables|Getstart%20position) (LocalVariables|Getlook%20target))) (.yaw (Math|Rotator|FindLookatRotation (LocalVariables|Getstart%20position) (LocalVariables|Getlook%20target)))) 1.0)))))))
            (:then_3
              (return (LocalVariables|Getdone%20rotate) (LocalVariables|GetInterp%20Output)))))
        (:else)))))

(fn SameinArray?
  (params (Array :type Array%20of%20Actor%20Object%20References) (Object :type Actor%20Object%20Reference))
  (Utilities|IsValid (Utilities|Array|Get(acopy) Array (Utilities|Array|FindItem Array Object))
    (:Is%20Valid
      (LocalVariables|Setoutput true))
    (:Is%20Not%20Valid
      (LocalVariables|Setoutput false)))
  (return (LocalVariables|Getoutput)))

(fn ArrayLength
  (params (Array :type Array%20of%20Actor%20Object%20References))
  (return (Math|Conversions|ToBoolean(Integer) (Utilities|Array|Length Array))))