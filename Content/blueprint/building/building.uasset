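; Base Blueprint for grid-placed buildings (blocks, turrets, mines), dispatching to the child class by BuildIndex.
; Construction applies a custom-depth preview material; ApplyBlockSet swaps in final materials, sets high-cost enemy nav area and runs type setup.
; Non-friendly damage is reduced by armor; at zero health, upward traces destroy cells and buildings stacked above.
; Destruction resets nav area, frees the traced cell below, then fades opacity after a delay before removing the actor.
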(event Custom|parent:AnyDamage
  (params (damage%20type :type Damage%20Type%20Object%20Reference) (damage :type Float%20%28single-precision%29))
  (bind _self self)
  (bind _health_0_ (Utilities|CalculateDamage damage%20type damage))
  (if _health_0_
    (CallFunction|CheckObjectOver)
    (Variables|Default|Setbrocken? true)
    (Class|NavModifierComponent|SetAreaClass (Variables|Default|Getcorner%20cut))
    (bind _cell_hit (CallFunction|CheckCellUnder))
    (bind _asgrid (Utilities|Casting|CastTogrid _cell_hit)
      (:then
        (Variables|/Game/blueprint/building/grid/grid.grid_C|Setstate_grid _asgrid 0)
        (Utilities|FlowControl|Sequence
          (:then_0
            (switch int (Variables|Default|Getbuild%20index)
              (:1
                (bind _asblock (Utilities|Casting|CastToblock _self))
                (bind _block_m (Default|DestroytheBlock _asblock))
                (Variables|Setup|Setmaterial%20brush%201 _block_m))
              (:2
                (bind _asturret_base (Utilities|Casting|CastToturret_base _self))
                (bind (_head_m _body_m) (Default|KillTurret _asturret_base))
                (Variables|Setup|Setmaterial%20brush%201 _head_m)
                (Variables|Setup|Setmaterial%20brush%202 _body_m))
              (:3
                (bind _asmine (Utilities|Casting|CastTomine _self))
                (switch int (Variables|/Game/blueprint/building/mine/mine.mine_C|Getlvl _asmine)
                  (:Default
                    (Development|PrintString "no lvl mine(destroing)"))
                  (:1
                    (bind _asmine_1_lvl (Utilities|Casting|CastTomine_1_lvl _asmine))
                    (bind _all_mine (Default|Kill1LvlMine _asmine_1_lvl))
                    (Variables|Setup|Setmaterial%20brush%201 _all_mine))))))
          (:then_1
            (Utilities|Time|SetTimerbyEvent (delegate Custom|end%20of%20killing) 3.0))))
      (:CastFailed
        (Development|PrintString "no cell under(destroy build)")))))

(event Custom|end%20of%20killing
  (bind _newtrack_0 (Timeline|Timeline_0 PlayFromStart)
    (:Update
      (bind _material_brush_1 (Variables|Setup|Getmaterial%20brush%201)
        (:then
          (Rendering|Material|SetScalarParameterValue _material_brush_1 "opacity" _newtrack_0 :!class /Script/Engine.MaterialInstanceDynamic))
        (:else
          _))
      (bind _material_brush_2 (Variables|Setup|Getmaterial%20brush%202)
        (:then
          (Rendering|Material|SetScalarParameterValue _material_brush_2 "opacity" _newtrack_0 :!class /Script/Engine.MaterialInstanceDynamic))
        (:else)))
    (:Finished
      (Actor|DestroyActor))))

(event Custom|apply%20block%20set
  (bind _self self)
  (Rendering|Components|TextRender|SetText (Variables|Default|Gethealth%20building) (Utilities|Text|ToText(Float) (Variables|Default|Gethealth) "HalfToEven"))
  (Class|NavModifierComponent|SetAreaClass (Variables|Default|Getcorner%20cut) "/Game/blueprint/enemies_bp/navigation/enemys_high_cost_nav.enemys_high_cost_nav_C")
  (Utilities|FlowControl|Sequence
    (:then_0
      (bind _mesh_element_1 (Variables|Setup|Getmesh%20element%201)
        (:then
          (Rendering|Material|SetMaterial _mesh_element_1 0 (Variables|Setup|Getmaterial%20element%201))
          (Rendering|SetRenderCustomDepth _mesh_element_1 false))
        (:else)))
    (:then_1
      (bind _mesh_element_2 (Variables|Setup|Getmesh%20element%202)
        (:then
          (Rendering|Material|SetMaterial _mesh_element_2 0 (Variables|Setup|Getmaterial%20element%202))
          (Rendering|SetRenderCustomDepth _mesh_element_2 false))
        (:else)))
    (:then_2
      (bind _skeletal_mesh_1 (Variables|Default|Getskeletal%20mesh%201)
        (:then
          (Rendering|Material|SetMaterial _skeletal_mesh_1 0 (Variables|Setup|Getskeletal%20material%201))
          (Rendering|SetRenderCustomDepth _skeletal_mesh_1 false))
        (:else)))
    (:then_3
      (switch int (Variables|Default|Getbuild%20index)
        (:2
          (bind _asturret_base (Utilities|Casting|CastToturret_base _self))
          (Default|StartSetup _asturret_base))
        (:3
          (bind _asmine (Utilities|Casting|CastTomine _self))
          (Default|Setup _asmine))))))

(event Custom|destroy%20building
  (bind _self self)
  (Variables|Default|Setbrocken? true)
  (Class|NavModifierComponent|SetAreaClass (Variables|Default|Getcorner%20cut))
  (bind _cell_hit (CallFunction|CheckCellUnder))
  (bind _asgrid (Utilities|Casting|CastTogrid _cell_hit)
    (:then
      (Variables|/Game/blueprint/building/grid/grid.grid_C|Setstate_grid _asgrid 0)
      (Utilities|FlowControl|Sequence
        (:then_0
          (switch int (Variables|Default|Getbuild%20index)
            (:1
              (bind _asblock (Utilities|Casting|CastToblock _self))
              (bind _block_m (Default|DestroytheBlock _asblock))
              (Variables|Setup|Setmaterial%20brush%201 _block_m))
            (:2
              (bind _asturret_base (Utilities|Casting|CastToturret_base _self))
              (bind (_head_m _body_m) (Default|KillTurret _asturret_base))
              (Variables|Setup|Setmaterial%20brush%201 _head_m)
              (Variables|Setup|Setmaterial%20brush%202 _body_m))
            (:3
              (bind _asmine (Utilities|Casting|CastTomine _self))
              (switch int (Variables|/Game/blueprint/building/mine/mine.mine_C|Getlvl _asmine)
                (:Default
                  (Development|PrintString "no lvl mine(destroing)"))
                (:1
                  (bind _asmine_1_lvl (Utilities|Casting|CastTomine_1_lvl _asmine))
                  (bind _all_mine (Default|Kill1LvlMine _asmine_1_lvl))
                  (Variables|Setup|Setmaterial%20brush%201 _all_mine))))))
        (:then_1
          (Utilities|Time|SetTimerbyEvent (delegate Custom|end%20of%20killing) 3.0))))
    (:CastFailed
      (Development|PrintString "no cell under(destroy build)"))))

(event EventBeginPlay
  (bind _ascharacter_bp (Utilities|Casting|CastTocharacter_bp (Game|Player|GetPlayerPawn 0)))
  (Variables|Default|Setplayer_ref _ascharacter_bp))

(event Collision|EventActorBeginOverlap
  (params (OtherActor :type Actor%20Object%20Reference)))

(event EventTick
  (params (DeltaSeconds :type Float%20%28single-precision%29))
  (Utilities|Casting|CastTomain_game_mode (Game|GetGameMode)))

(fn ConstructionScript
  (bind _asmain_game_mode (Utilities|Casting|CastTomain_game_mode (Game|GetGameMode)))
  (Variables|Default|Setgame_mode _asmain_game_mode)
  (Class|NavModifierComponent|SetAreaClass (Variables|Default|Getcorner%20cut))
  (Utilities|FlowControl|Sequence
    (:then_0
      (bind _mesh_element_1 (Variables|Setup|Getmesh%20element%201)
        (:then
          (Rendering|Material|SetMaterial _mesh_element_1 0 "/Game/assets/game/outline/buildings.buildings")
          (Rendering|SetRenderCustomDepth _mesh_element_1 true)
          (Rendering|SetCustomDepthStencilValue _mesh_element_1 2))
        (:else)))
    (:then_1
      (bind _mesh_element_2 (Variables|Setup|Getmesh%20element%202)
        (:then
          (Rendering|Material|SetMaterial _mesh_element_2 0 "/Game/assets/game/outline/buildings.buildings")
          (Rendering|SetRenderCustomDepth _mesh_element_2 true)
          (Rendering|SetCustomDepthStencilValue _mesh_element_2 2))
        (:else)))
    (:then_2
      (bind _skeletal_mesh_1 (Variables|Default|Getskeletal%20mesh%201)
        (:then
          (Rendering|Material|SetMaterial _skeletal_mesh_1 0 "/Game/assets/game/outline/buildings.buildings")
          (Rendering|SetRenderCustomDepth _skeletal_mesh_1 true)
          (Rendering|SetCustomDepthStencilValue _skeletal_mesh_1 2))
        (:else)))))

(fn CheckCellUnder
  (bind _center (Variables|Default|Getcenter))
  (bind _returnvalue (Transformation|GetWorldLocation _center))
  (bind _outhit (Collision|LineTraceForObjects (Math|Vector|MakeVector (.x _returnvalue) (.y _returnvalue) (.z _returnvalue)) (Math|Vector|MakeVector (.x _returnvalue) (.y _returnvalue) (- (.z _returnvalue) 1e+04)) (Utilities|Array|MakeArray "ObjectTypeQuery10") false 0 "None"))
  (return (.Location (Collision|BreakHitResult _outhit)) (.HitActor (Collision|BreakHitResult _outhit))))

(fn CheckObjectOver
  (bind _center (Variables|Default|Getcenter))
  (bind _returnvalue (Transformation|GetWorldLocation _center))
  (bind _outhits (Class|KismetSystemLibrary|LineTraceMultiforObjects (Math|Vector|MakeVector (.x _returnvalue) (.y _returnvalue) (.z _returnvalue)) (Math|Vector|MakeVector (.x _returnvalue) (.y _returnvalue) (+ (.z _returnvalue) 1e+04)) (Utilities|Array|MakeArray "ObjectTypeQuery10" "ObjectTypeQuery1" "ObjectTypeQuery8") false 0 "ForOneFrame" true "(R=0.000191,G=0.000000,B=1.000000,A=1.000000)"))
  (for _array_element _outhits
    (bind _asgrid (Utilities|Casting|CastTogrid (.HitActor (Collision|BreakHitResult _array_element)))
      (:then
        (Utilities|Array|RemoveItem (Variables|/Game/blueprint/character_bp/character_bp.character_bp_C|Getcell_elements_array (Variables|Default|Getplayer_ref)) _asgrid)
        (Actor|DestroyActor _asgrid))
      (:CastFailed
        (bind _asbuilding (Utilities|Casting|CastTobuilding (.HitActor (Collision|BreakHitResult _array_element))))
        (CallFunction|DestroyBuilding _asbuilding))))
  (return))

(fn GetFloor
  (bind _cell_hit (CallFunction|CheckCellUnder))
  (bind _asgrid (Utilities|Casting|CastTogrid _cell_hit))
  (return (Variables|/Game/blueprint/building/grid/grid.grid_C|Getfloor%20number _asgrid)))