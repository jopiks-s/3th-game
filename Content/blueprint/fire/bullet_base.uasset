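; Base projectile Blueprint that moves at a configurable bullet speed and deals damage to whatever its Box collider hits.
; The construction script applies the speed to ProjectileMovement.
; On spawn it ignores its damage causer, plays a shot sound, caches the player character and sets its lifespan.
; On hit it applies typed damage, disables collision, hides itself and destroys itself after a short delay.
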(event OnComponentHit(Box)
  (params (HitComponent :type Primitive%20Component%20Object%20Reference) (OtherActor :type Actor%20Object%20Reference) (OtherComp :type Primitive%20Component%20Object%20Reference) (NormalImpulse :type Vector :default "0, 0, 0") (Hit :type Hit%20Result%20Structure%20%28by%20ref%29))
  (bind _box (Variables|Pawn|GetBox))
  (Game|Damage|ApplyDamage OtherActor (Variables|Default|Getdamage) 0 (Variables|Default|Getdamage%20causer) (Variables|Default|Getdamage_type))
  (Collision|SetCollisionEnabled _box "NoCollision")
  (Development|SetHiddeninGame _box true true)
  (Development|SetHiddeninGame (Variables|Default|GetStaticMesh) true true)
  (Utilities|FlowControl|Delay 1.0)
  (Actor|DestroyActor))

(event EventBeginPlay
  (Collision|IgnoreActorwhenMoving (Variables|Pawn|GetBox) (Variables|Default|Getdamage%20causer) true)
  (Audio|PlaySoundatLocation "/Game/assets/game/audio/shoot.shoot" (Transformation|GetActorLocation) "0, 0, 0" 1.0 1.0 0.0 0 0 0)
  (bind _ascharacter_bp (Utilities|Casting|CastTocharacter_bp (Game|Player|GetPlayerPawn 0)))
  (Variables|Default|Setplayer_ref _ascharacter_bp)
  (Actor|SetLifeSpan (Variables|Default|Getlife%20span)))

(fn ConstructionScript
  (bind _projectilemovement (Variables|Default|GetProjectileMovement))
  (bind _bullet_speed (Variables|Default|Getbullet_speed))
  (Variables|/Script/Engine.ProjectileMovementComponent|SetInitialSpeed _projectilemovement _bullet_speed)
  (Variables|/Script/Engine.ProjectileMovementComponent|SetMaxSpeed _projectilemovement _bullet_speed))