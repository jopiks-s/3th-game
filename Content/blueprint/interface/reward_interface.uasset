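; Floating reward text actor that displays a given string, drifts upward, fades out and destroys itself.
; The construction script randomizes the text's X and Y scale, sets the string, then calls Move.
; Move creates a dynamic text material, caches the player character and runs two chained timelines.
; The first raises the actor by a fixed step per update; the second keeps it rising while animating opacity, then destroys it.
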(event Custom|move
  (bind _returnvalue (Rendering|Material|CreateDynamicMaterialInstance (Variables|Default|GetTextRender) 0 "/Engine/EngineMaterials/DefaultTextMaterialOpaque_Inst.DefaultTextMaterialOpaque_Inst" "None" :!class /Script/Engine.PrimitiveComponent))
  (bind _ascharacter_bp (Utilities|Casting|CastTocharacter_bp (Game|Player|GetPlayerPawn 0)))
  (Variables|Default|Setcharacter _ascharacter_bp)
  (Timeline|ss PlayFromStart
    (:Update
      (Transformation|AddWorldOffset (Variables|Default|GetDefaultSceneRoot) "0, 0,0.760000" false false :!label _label))
    (:Finished
      (bind _newtrack_2 (Timeline|Timeline_0 PlayFromStart)
        (:Update
          (Rendering|Material|SetScalarParameterValue _returnvalue "opacity" _newtrack_2 :!class /Script/Engine.MaterialInstanceDynamic)
          (goto _label))
        (:Finished
          (Actor|DestroyActor))))))

(event EventBeginPlay)

(event Collision|EventActorBeginOverlap
  (params (OtherActor :type Actor%20Object%20Reference)))

(event EventTick
  (params (DeltaSeconds :type Float%20%28single-precision%29)))

(fn ConstructionScript
  (bind _returnvalue (Math|Random|RandomFloatinRange 1.6 2.0))
  (bind _textrender (Variables|Default|GetTextRender))
  (Rendering|Components|TextRender|SetXScale _textrender _returnvalue)
  (Rendering|Components|TextRender|SetYScale _textrender _returnvalue)
  (Rendering|Components|TextRender|SetText _textrender (Variables|Default|Gettext%20))
  (CallFunction|Move))